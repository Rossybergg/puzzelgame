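; Memory is a spinning collectable that the first-person player picks up to unlock the level's exit.
; Each instance adds one to MemoryUI's needed count at BeginPlay, using the widget's text fields as the counters.
; Its first player overlap increments the collected count, flashes the UI, triggers sounds, hides it and destroys it after a delay.
; When the counts match, it also plays an unlock sound, then turns the first ExitDoor green and opens it.
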(event `self.ReceiveBeginPlay`
  (`|ExecutionSequence`
    (:`then_0`
      (bind (_direction _newtrack_0) (`Timeline|Rotation`)
        (:`Update`
          (`SceneComponent.K2_SetWorldRotation` (`self.memory`) (`KismetMathLibrary.MakeRotator` 0.0 _newtrack_0 _newtrack_0) false false))))
    (:`then_1`
      (`KismetSystemLibrary.Delay` 0.0)
      (bind _foundwidgets (`WidgetBlueprintLibrary.GetAllWidgetsOfClass` "/Game/Collectables/Blueprints/MemoryUI.MemoryUI_C"))
      (bind _memoriesneeded (`/Game/Collectables/Blueprints/MemoryUI.MemoriesNeeded` (`|GetArrayItem` _foundwidgets)))
      (`TextBlock.SetText` _memoriesneeded (`KismetTextLibrary.Conv_IntToText` (+ (`KismetStringLibrary.Conv_StringToInt` (`KismetTextLibrary.Conv_TextToString` (`TextBlock.GetText` _memoriesneeded))) 1))))))

(event `self.Box.OnComponentBeginOverlap`
  (params (OverlappedComponent :type "PrimitiveComponent Object Reference") (OtherActor :type "Actor Object Reference") (OtherComp :type "PrimitiveComponent Object Reference") (OtherBodyIndex :type Integer) (bFromSweep :type Boolean) (SweepResult :type "HitResult Structure (by ref)"))
  (cast `/Game/FirstPerson/Blueprints/BP_FirstPersonCharacter` OtherActor)
  (`/Engine/EditorBlueprintResources/StandardMacros.DoOnce` false
    (:`Completed`
      (bind _foundwidgets (`WidgetBlueprintLibrary.GetAllWidgetsOfClass` "/Game/Collectables/Blueprints/MemoryUI.MemoryUI_C"))
      (bind _output (`|GetArrayItem` _foundwidgets))
      (bind _memoriescollected (`/Game/Collectables/Blueprints/MemoryUI.MemoriesCollected` _output))
      (bind _returnvalue (`TextBlock.GetText` _memoriescollected))
      (`TextBlock.SetText` _memoriescollected (`KismetTextLibrary.Conv_IntToText` (+ (`KismetStringLibrary.Conv_StringToInt` (`KismetTextLibrary.Conv_TextToString` _returnvalue)) 1)))
      (if (`KismetTextLibrary.EqualEqual_TextText` _returnvalue (`TextBlock.GetText` (`/Game/Collectables/Blueprints/MemoryUI.MemoriesNeeded` _output)))
        (bind _outactors (`GameplayStatics.GetAllActorsOfClass` "/Game/Collectables/Blueprints/ExitDoor.ExitDoor_C"))
        (`|ExecutionSequence`
          (:`then_0`
            (bind _output_2 (`|GetArrayItem` (stale `self.ReceiveBeginPlay` _foundwidgets)))
            (`UserWidget.PlayAnimation` _output_2 (`/Game/Collectables/Blueprints/MemoryUI.MemoryFlash` _output_2) 0.0 1 "Forward" 1.0 false :!label _label)
            (`ActorComponent.Activate` (`self.Memory Sound 2`) false)
            (`ActorComponent.Activate` (`self.Memory Sound 1`) false)
            (`self.SetActorHiddenInGame` true)
            (`KismetSystemLibrary.Delay` 5.0)
            (`self.K2_DestroyActor`))
          (:`then_1`
            (`GameplayStatics.PlaySound2D` "/Game/Collectables/Sounds/Door_Unlock.Door_Unlock" 1.0 1.0 0.0 null null)
            (`KismetSystemLibrary.Delay` 1.6)
            (bind _output_3 (`|GetArrayItem` _outactors))
            (`PrimitiveComponent.SetMaterial` (`/Game/Collectables/Blueprints/ExitDoor.Door` _output_3) 0 "/Game/Platforms/Materials/Green.Green")
            (set `/Game/Collectables/Blueprints/ExitDoor.open` true _output_3)))
        (else
          (goto _label))))))

(fn `UserConstructionScript`)